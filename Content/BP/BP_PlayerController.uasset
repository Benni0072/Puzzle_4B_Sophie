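; Player controller for the first-person character that routes Enhanced Input to the possessed pawn.
; On BeginPlay it adds the first-person mapping context, and on possess it caches the pawn as a first-person character.
; The move action drives the character's MoveInWorldDirection, and the camera action feeds its controller yaw and pitch.
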(event Input|EnhancedActionEvents|EnhancedInputActionIA_Move
  (params (ActionValue :type Vector%202D%20Structure) (ElapsedSeconds :type Float%20%28double-precision%29) (TriggeredSeconds :type Float%20%28double-precision%29) (InputAction :type Input%20Action%20Object%20Reference :default "/Game/Input/InputActions/IA_Move.IA_Move"))
  (:Triggered
    (Default|MoveinWorldDirection (Variables|Default|GetFirstPersonCharacter) (Math|Vector|MakeVector (.x ActionValue) (.y ActionValue) 0.0))))

(event Input|EnhancedActionEvents|EnhancedInputActionIA_MoveCamera
  (params (ActionValue :type Vector%202D%20Structure) (ElapsedSeconds :type Float%20%28double-precision%29) (TriggeredSeconds :type Float%20%28double-precision%29) (InputAction :type Input%20Action%20Object%20Reference :default "/Game/Input/InputActions/IA_MoveCamera.IA_MoveCamera"))
  (bind _firstpersoncharacter (Variables|Default|GetFirstPersonCharacter))
  (:Triggered
    (Pawn|Input|AddControllerYawInput _firstpersoncharacter (.x ActionValue))
    (Pawn|Input|AddControllerPitchInput _firstpersoncharacter (.y ActionValue))))

(event EventPossess
  (params (PossessedPawn :type Pawn%20Object%20Reference))
  (bind _asbp_first_person_character (Utilities|Casting|CastToBP_FirstPersonCharacter PossessedPawn))
  (Variables|Default|SetFirstPersonCharacter _asbp_first_person_character))

(event EventBeginPlay
  (Input|AddMappingContext (PlayerController|LocalPlayerSubsystems|GetEnhancedInputLocalPlayerSubsystem) "/Game/Input/IMC_FirstPerson.IMC_FirstPerson" 0 "(bIgnoreAllPressedKeysUntilRelease=True,bForceImmediately=False,bNotifyUserSettings=False)"))

(fn ConstructionScript)