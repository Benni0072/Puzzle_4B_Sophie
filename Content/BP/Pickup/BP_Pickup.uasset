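; BP_Pickup is an interactable item that the player picks up and can rotate while held.
; Interact snaps its Pickup component to the character's PickupPivot, keeping world scale, and disables its collision.
; RotateItem turns that pivot in world space by combining pitch around the actor's right vector with negated yaw, whose axis is a zero vector.
; The detach node is never executed, so the file has no working drop.
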(event EventInteract
  (params (PlayerCharacter :type BP%20First%20Person%20Character%20Object%20Reference))
  (Transformation|AttachComponentToComponent (Variables|Default|GetPickup) (Variables|/Game/BP/BP_FirstPersonCharacter.BP_FirstPersonCharacter_C|GetPickupPivot PlayerCharacter) "None" "SnapToTarget" "SnapToTarget" "KeepWorld" true)
  (Collision|SetCollisionEnabled (Variables|Default|GetPickup) "NoCollision"))

(fn ConstructionScript)

(fn RotateItem
  (Transformation|AddWorldRotation (Variables|/Game/BP/BP_FirstPersonCharacter.BP_FirstPersonCharacter_C|GetPickupPivot (Variables|Default|GetFirstPersonCharacter)) (Math|Rotator|CombineRotators (Math|Vector|RotatorfromAxisandAngle "0, 0, 0" (* (Variables|Default|GetYaw) -1.0)) (Math|Vector|RotatorfromAxisandAngle (Transformation|GetActorRightVector) (Variables|Default|GetPitch))) false false))