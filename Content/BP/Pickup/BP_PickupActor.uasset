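; BP_PickupActor is a physics object that can be picked up, carried and dropped.
; AttachTo disables physics and collision on the Pickup component and snaps it to a given component; Drop detaches it and restores both.
; RotateItem turns the first-person character's PickupPivot from yaw and pitch, using the actor's right vector for pitch and a zero axis for yaw.
; Interact is a stub returning false.
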(event Custom|AttachTo
  (params (ComponentToAttacheTo :type Scene%20Component%20Object%20Reference))
  ;[0.15 0.15 0.15 0.5] Keine Physik
  (Physics|SetSimulatePhysics (Variables|Default|GetPickup) false)
  ;[0.15 0.15 0.15 0.5] KeineCollision
  (Collision|SetCollisionEnabled (Variables|Default|GetPickup) "NoCollision")
  (Transformation|AttachComponentToComponent ComponentToAttacheTo "None" "SnapToTarget" "SnapToTarget" "KeepWorld" true))

(event Custom|Drop
  ;[0.15 0.15 0.15 0.5] Object fallen lassen
  (Transformation|DetachFromActor "KeepWorld" "KeepWorld" "KeepWorld")
  (Collision|SetCollisionEnabled (Variables|Default|GetPickup) "QueryAndPhysics")
  (Physics|SetSimulatePhysics (Variables|Default|GetPickup) true))

(fn ConstructionScript)

(fn RotateItem
  (Transformation|AddWorldRotation (Variables|/Game/BP/BP_FirstPersonCharacter.BP_FirstPersonCharacter_C|GetPickupPivot (Variables|Default|GetFirstPersonCharacter)) (Math|Rotator|CombineRotators (Math|Vector|RotatorfromAxisandAngle "0, 0, 0" (* (Variables|Default|GetYaw) -1.0)) (Math|Vector|RotatorfromAxisandAngle (Transformation|GetActorRightVector) (Variables|Default|GetPitch))) false false))

(fn Interact
  (params (PlayerCharacter :type BP%20First%20Person%20Character%20Object%20Reference) (Pickup :type BP%20Pickup%20Actor%20Object%20Reference))
  (return false))