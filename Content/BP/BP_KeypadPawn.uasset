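; Possessable keypad puzzle pawn where the player enters a code on twelve buttons.
; Interact possesses it and swaps first-person input for puzzle input; exiting reverses both.
; Navigation steps a wrapping index through the button array by one or three for grid movement, highlighting via overlay material.
; The TextRender doubles as the entry buffer checked against CorrectCode; a correct code only returns control, with unlocking left as a comment.
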(event Input|EnhancedActionEvents|EnhancedInputActionIA_ExitPuzzle
  (params (ActionValue :type Boolean) (ElapsedSeconds :type Float%20%28double-precision%29) (TriggeredSeconds :type Float%20%28double-precision%29) (InputAction :type Input%20Action%20Object%20Reference :default "/Game/Input/InputActions/IA_ExitPuzzle.IA_ExitPuzzle"))
  ;[1 1 1] Posess / Unposess
  (CallFunction|ReturntoPlayerCHaracter))

(event Input|EnhancedActionEvents|EnhancedInputActionIA_NavigateRight
  (params (ActionValue :type Boolean) (ElapsedSeconds :type Float%20%28double-precision%29) (TriggeredSeconds :type Float%20%28double-precision%29) (InputAction :type Input%20Action%20Object%20Reference :default "/Game/Input/InputActions/IA_NavigateRight.IA_NavigateRight"))
  ;[1 1 1] Highlight Navigation
  (CallFunction|NavigateButtons 1))

(event Input|EnhancedActionEvents|EnhancedInputActionIA_NavigateLeft
  (params (ActionValue :type Boolean) (ElapsedSeconds :type Float%20%28double-precision%29) (TriggeredSeconds :type Float%20%28double-precision%29) (InputAction :type Input%20Action%20Object%20Reference :default "/Game/Input/InputActions/IA_NavigateLeft.IA_NavigateLeft"))
  ;[1 1 1] Highlight Navigation
  (CallFunction|NavigateButtons -1))

(event Input|EnhancedActionEvents|EnhancedInputActionIA_NavigateUp
  (params (ActionValue :type Boolean) (ElapsedSeconds :type Float%20%28double-precision%29) (TriggeredSeconds :type Float%20%28double-precision%29) (InputAction :type Input%20Action%20Object%20Reference :default "/Game/Input/InputActions/IA_NavigateUp.IA_NavigateUp"))
  ;[1 1 1] Highlight Navigation
  (CallFunction|NavigateButtons -3))

(event Input|EnhancedActionEvents|EnhancedInputActionIA_NavigateDown
  (params (ActionValue :type Boolean) (ElapsedSeconds :type Float%20%28double-precision%29) (TriggeredSeconds :type Float%20%28double-precision%29) (InputAction :type Input%20Action%20Object%20Reference :default "/Game/Input/InputActions/IA_NavigateDown.IA_NavigateDown"))
  ;[1 1 1] Highlight Navigation
  (CallFunction|NavigateButtons 3))

(event Input|EnhancedActionEvents|EnhancedInputActionIA_Interact
  (params (ActionValue :type Boolean) (ElapsedSeconds :type Float%20%28double-precision%29) (TriggeredSeconds :type Float%20%28double-precision%29) (InputAction :type Input%20Action%20Object%20Reference :default "/Game/Input/InputActions/IA_Interact.IA_Interact"))
  (if (== (CallFunction|GetSelectedButton) (Variables|Default|GetButton_Confirm))
    ;[1 1 1] Check if Code Correct
    (if (CallFunction|IsCodeCorrect)
      ;;[1 1 1] Unlock secret / open door
      (CallFunction|ReturntoPlayerCHaracter)
      (else
        (CallFunction|ClearDisplay)))
    (elif (== (CallFunction|GetSelectedButton) (Variables|Default|GetButton_Cancle))
      (CallFunction|ClearDisplay)
      (elif (not (CallFunction|IsCodeComplete))
        (CallFunction|AddtoDisplay (Variables|/Game/BP/BP_KeypadButton.BP_KeypadButton_C|GetButtonLabel (CallFunction|GetSelectedButton)))))))

(event EventInteract
  (params (PlayerCharacter :type BP%20First%20Person%20Character%20Object%20Reference))
  ;[1 1 1] Posess / Unposess
  (Variables|Default|SetPlayerCharacter PlayerCharacter)
  (Pawn|Possess (Game|GetPlayerController 0) self)
  ;;[1 1 1] Vergiss FirstPerson Steueerung
  (Input|RemoveMappingContext (PlayerController|LocalPlayerSubsystems|GetEnhancedInputLocalPlayerSubsystem (Game|GetPlayerController 0)) "/Game/Input/IMC_FirstPerson.IMC_FirstPerson" "(bIgnoreAllPressedKeysUntilRelease=True,bForceImmediately=False,bNotifyUserSettings=False)")
  ;;[1 1 1] Bekomme die Puzzle Steuerung
  (Input|AddMappingContext (PlayerController|LocalPlayerSubsystems|GetEnhancedInputLocalPlayerSubsystem (Game|GetPlayerController 0)) "/Game/Input/IMC_Puzzle.IMC_Puzzle" 0 "(bIgnoreAllPressedKeysUntilRelease=True,bForceImmediately=False,bNotifyUserSettings=False)")
  (CallFunction|UpdateHighlightOfSelectedButton true))

(event EventBeginPlay
  ;[1 1 1] Setup
  (Variables|Default|SetButtons (Utilities|Array|MakeArray (Variables|Default|GetButton_1) (Variables|Default|GetButton_2) (Variables|Default|GetButton_3) (Variables|Default|GetButton_4) (Variables|Default|GetButton_5) (Variables|Default|GetButton_6) (Variables|Default|GetButton_7) (Variables|Default|GetButton_8) (Variables|Default|GetButton_9) (Variables|Default|GetButton_Cancle) (Variables|Default|GetButton_0) (Variables|Default|GetButton_Confirm)))
  (CallFunction|ClearDisplay))

(fn ConstructionScript)

(fn GetSelectedButton
  (return (Utilities|Array|Get(acopy) (Variables|Default|GetButtons) (Variables|Default|GetCurrentButtonIndex))))

(fn UpdateHighlightOfSelectedButton
  (params (Enable :type Boolean))
  (Rendering|Material|SetOverlayMaterial (CallFunction|GetSelectedButton) (select Enable "/Game/Material/MM_Highlight_Inst.MM_Highlight_Inst" 0) :!class /Script/Engine.MeshComponent))

(fn NavigateButtons
  (params (Direction :type Integer))
  (CallFunction|UpdateHighlightOfSelectedButton false)
  (Variables|Default|SetCurrentButtonIndex (+ (Variables|Default|GetCurrentButtonIndex) Direction))
  (Utilities|FlowControl|Sequence
    (:then_0
      ;[1 1 1] Check if to high
      (if (> (Variables|Default|GetCurrentButtonIndex) (Utilities|Array|LastIndex (Variables|Default|GetButtons)))
        (Variables|Default|SetCurrentButtonIndex (- (Variables|Default|GetCurrentButtonIndex) (Utilities|Array|Length (Variables|Default|GetButtons))))))
    (:then_1
      ;[1 1 1] Check if to low
      (if (< (Variables|Default|GetCurrentButtonIndex) 0)
        (Variables|Default|SetCurrentButtonIndex (+ (Variables|Default|GetCurrentButtonIndex) (Utilities|Array|Length (Variables|Default|GetButtons))))))
    (:then_2
      ;[1 1 1] Update Highlight
      (CallFunction|UpdateHighlightOfSelectedButton true))))

(fn ClearDisplay
  (Rendering|Components|TextRender|SetText (Variables|Default|GetTextRender) (Utilities|Text|ToText(String) "")))

(fn AddtoDisplay
  (params (B :type String))
  (bind _textrender (Variables|Default|GetTextRender))
  (Rendering|Components|TextRender|SetText _textrender (Utilities|Text|ToText(String) (Utilities|String|Append (Utilities|String|ToString(Text) (Variables|/Script/Engine.TextRenderComponent|GetText _textrender)) B))))

(fn IsCodeComplete
  (return (== (Utilities|String|Len (Utilities|String|ToString(Text) (Variables|/Script/Engine.TextRenderComponent|GetText (Variables|Default|GetTextRender)))) (Utilities|String|Len (Variables|Default|GetCorrectCode)))))

(fn IsCodeCorrect
  (return (Utilities|Enum|Equal(Enum) (Utilities|String|ToString(Text) (Variables|/Script/Engine.TextRenderComponent|GetText (Variables|Default|GetTextRender))) (Variables|Default|GetCorrectCode))))

(fn ReturntoPlayerCHaracter
  (Input|RemoveMappingContext (PlayerController|LocalPlayerSubsystems|GetEnhancedInputLocalPlayerSubsystem (Game|GetPlayerController 0)) "/Game/Input/IMC_Puzzle.IMC_Puzzle" "(bIgnoreAllPressedKeysUntilRelease=True,bForceImmediately=False,bNotifyUserSettings=False)")
  (Input|AddMappingContext (PlayerController|LocalPlayerSubsystems|GetEnhancedInputLocalPlayerSubsystem (Game|GetPlayerController 0)) "/Game/Input/IMC_FirstPerson.IMC_FirstPerson" 0 "(bIgnoreAllPressedKeysUntilRelease=True,bForceImmediately=False,bNotifyUserSettings=False)")
  (Pawn|Possess (Game|GetPlayerController 0) (Variables|Default|GetPlayerCharacter))
  (CallFunction|UpdateHighlightOfSelectedButton false))