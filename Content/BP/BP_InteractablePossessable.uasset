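; Base interactable pawn that the player can possess, swapping first-person character controls for puzzle controls and back.
; Interacting, if allowed, swaps Enhanced Input mapping contexts and blends the view before possession, with a fixed one-second delay; ReturnToCharacter reverses this.
; PositionPlayer aligns the character to a child-supplied camera's rotation and floor-traced location.
; SetHighlight toggles an overlay highlight material on a given mesh.
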(event Custom|ReturnToCharacter
  ;[1 1 1] Possess Character
  (Input|RemoveMappingContext (PlayerController|LocalPlayerSubsystems|GetEnhancedInputLocalPlayerSubsystem (Game|GetPlayerController 0)) (Variables|Default|GetMapping%20Context) "(bIgnoreAllPressedKeysUntilRelease=True,bForceImmediately=False,bNotifyUserSettings=False)")
  (Game|Player|SetViewTargetwithBlend (Game|GetPlayerController 0) (Variables|Default|GetPlayer%20Character) (Variables|Default|GetSmoothPossesssDuration) "VTBlend_Linear" 0.0 false)
  (Utilities|FlowControl|Delay 1.0)
  (Input|AddMappingContext (PlayerController|LocalPlayerSubsystems|GetEnhancedInputLocalPlayerSubsystem (Game|GetPlayerController 0)) (Variables|Default|GetCharacterMapping%20Context) 0 "(bIgnoreAllPressedKeysUntilRelease=True,bForceImmediately=False,bNotifyUserSettings=False)")
  (Pawn|Possess (Game|GetPlayerController 0) (Variables|Default|GetPlayer%20Character)))

(event Custom|GetPossessed
  ;[1 1 1] Get Possessed
  ;;[1 1 1] Vergiss FirstPerson Steueerung
  (Input|RemoveMappingContext (PlayerController|LocalPlayerSubsystems|GetEnhancedInputLocalPlayerSubsystem (Game|GetPlayerController 0)) (Variables|Default|GetCharacterMapping%20Context) "(bIgnoreAllPressedKeysUntilRelease=True,bForceImmediately=False,bNotifyUserSettings=False)")
  (Game|Player|SetViewTargetwithBlend (Game|GetPlayerController 0) self (Variables|Default|GetSmoothPossesssDuration) "VTBlend_Linear" 0.0 false)
  (Utilities|FlowControl|Delay 1.0)
  (Pawn|Possess (Game|GetPlayerController 0) self)
  ;;[1 1 1] Bekomme die Puzzle Steuerung
  (Input|AddMappingContext (PlayerController|LocalPlayerSubsystems|GetEnhancedInputLocalPlayerSubsystem (Game|GetPlayerController 0)) (Variables|Default|GetMapping%20Context) 0 "(bIgnoreAllPressedKeysUntilRelease=True,bForceImmediately=False,bNotifyUserSettings=False)"))

(event EventInteract
  (params (PlayerCharacter :type BP%20First%20Person%20Character%20Object%20Reference))
  ;[1 1 1] Get Interact with
  (Variables|Default|SetPlayer%20Character PlayerCharacter)
  (if (Variables|Default|GetCanBePosssessed)
    (CallFunction|GetPossessed)))

(fn ConstructionScript)

(fn PositionPlayer
  (bind _output_get (LocalVariables|SetCam (Actor|GetComponentbyClass "/Script/Engine.CameraComponent")))
  (Utilities|IsValid _output_get
    (:Is%20Valid
      (Transformation|SetActorRotation (Variables|Default|GetPlayer%20Character) (Transformation|GetWorldRotation (LocalVariables|GetCam)))
      (bind _outhit (Collision|LineTraceForObjects (Transformation|GetWorldLocation (LocalVariables|GetCam)) (- (Transformation|GetWorldLocation (LocalVariables|GetCam)) "0.000000,0.000000,300.000000") (Utilities|Array|MakeArray "ObjectTypeQuery1" "ObjectTypeQuery2") false 0 "None"))
      (if true
        (Transformation|SetActorLocation (Variables|Default|GetPlayer%20Character) (+ (.Location (Collision|BreakHitResult _outhit)) (Math|Vector|MakeVector 0.0 0.0 (Variables|/Script/Engine.CapsuleComponent|GetCapsuleHalfHeight (Variables|/Script/Engine.Character|GetCapsuleComponent (Variables|Default|GetPlayer%20Character))))) false false)))
    (:Is%20Not%20Valid
      (Development|PrintString "BP_InteractablePossessable assumess child has camera component but found none!" true true "(R=1.000000,G=0.041157,B=0.313740,A=1.000000)"))))

(fn SetHighlight
  (params (Enable :type Boolean) (MeshComponent :type Mesh%20Component%20Object%20Reference))
  (Rendering|Material|SetOverlayMaterial MeshComponent (select Enable "/Game/Material/Highlight/MM_Highlight_Inst.MM_Highlight_Inst" 0) :!class /Script/Engine.MeshComponent))