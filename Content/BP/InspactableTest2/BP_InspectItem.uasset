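; BP_InspectItem is an inspectable item actor that shows a description widget while it is being inspected.
; It caches its transform on BeginPlay, and StartInspection creates BPW_Inspect with the item's description, character name and emotion image.
; EndInspection restores the cached transform and removes the widget; moving the item for inspection is not done here.
; Cursor hover only prints a debug string, and the node enabling mouse-over events is unconnected.
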(event OnBeginCursorOver(Item)
  (params (TouchedComponent :type Primitive%20Component%20Object%20Reference))
  (Development|PrintString "Hello"))

(event Custom|StartInspection
  (bind _returnvalue (UserInterface|CreateWidget "/Game/BP/Inspectables/BPW_Inspect.BPW_Inspect_C" (Game|GetPlayerController 0) (Variables|Default|GetItem%20Descr) (Variables|Default|GetCharacter%20Nam) (Variables|Default|GetNew%20Var)))
  (bind _output_get (Variables|Default|SetInspectWidgetRef _returnvalue))
  (UserInterface|Viewport|AddtoViewport _output_get 0))

(event Custom|EndInspection
  ;[0.15 0.15 0.15 0.5] Setze auf Location von vorher zurück
  (Transformation|SetActorTransform (Variables|Default|GetStartTransform))
  (Widget|RemovefromParent (Variables|Default|GetInspectWidgetRef)))

(event EventBeginPlay
  ;[0.15 0.15 0.15 0.5] Wenn Item aufgerufen wird set Location ItemPivot
  (Variables|Default|SetStartTransform (Transformation|GetActorTransform)))

(fn ConstructionScript)