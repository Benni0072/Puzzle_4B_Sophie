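; BP_Computer is an interactable computer in the computer puzzle that opens its screen UI when the player interacts with it.
; Interact switches input to UI only, shows the mouse cursor, and adds a new BPW_ComputerScreen widget to the viewport.
; It passes itself and its Referenz variable to the widget.
; Nodes that would remove the screen and restore game input are present but never run.
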(fn ConstructionScript)

(fn Interact
  (params (PlayerCharacter :type BP%20First%20Person%20Character%20Object%20Reference) (Pickup :type BP%20Pickup%20Actor%20Object%20Reference))
  (bind _returnvalue (Game|GetPlayerController 0))
  (Input|SetInputModeUIOnly _returnvalue 0 "DoNotLock" false)
  (bind _returnvalue_2 (UserInterface|CreateWidget "/Game/BP/ComputerPuzzle/BPW_ComputerScreen.BPW_ComputerScreen_C" _returnvalue))
  (bind _output_get (Variables|Default|SetBPW_Cpmputerscreen _returnvalue_2))
  (Variables|/Game/BP/ComputerPuzzle/BPW_ComputerScreen.BPW_ComputerScreen_C|SetBP_Computer _output_get self)
  (Variables|/Script/Engine.PlayerController|SetbShowMouseCursor (Game|GetPlayerController 0) true)
  (UserInterface|Viewport|AddtoViewport _output_get 0)
  (Variables|/Game/BP/ComputerPuzzle/BPW_ComputerScreen.BPW_ComputerScreen_C|SetBP_Referenz (Variables|Default|GetBPW_Cpmputerscreen) (Variables|Default|GetReferenz))
  (return false))