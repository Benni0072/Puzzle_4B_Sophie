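; BP_RotationPuzzle is an interactable three-disc combination puzzle, built on a parent class that supplies the interact and return-to-character logic.
; Navigation inputs move a highlighted selection along the discs, clamped at both ends, and rotate the selected disc either way.
; Interact input compares each disc's current symbol with CorrectCombination, printing the result and returning to the character only when all match.
; Exiting the puzzle clears the highlight.
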(event Input|EnhancedActionEvents|EnhancedInputActionIA_Interact
  (params (ActionValue :type Boolean) (ElapsedSeconds :type Float%20%28double-precision%29) (TriggeredSeconds :type Float%20%28double-precision%29) (InputAction :type Input%20Action%20Object%20Reference :default "/Game/Input/InputActions/IA_Interact.IA_Interact"))
  (if (CallFunction|EvaluateCombination)
    (Development|PrintString "Correct!" true true "(R=0.038914,G=0.385417,B=0.026096,A=1.000000)")
    (CallFunction|ReturntoCharacter)
    (else
      (Development|PrintString "Wrong!" true true "(R=0.515625,G=0.036996,B=0.026737,A=1.000000)"))))

(event Input|EnhancedActionEvents|EnhancedInputActionIA_ExitPuzzle
  (params (ActionValue :type Boolean) (ElapsedSeconds :type Float%20%28double-precision%29) (TriggeredSeconds :type Float%20%28double-precision%29) (InputAction :type Input%20Action%20Object%20Reference :default "/Game/Input/InputActions/IA_ExitPuzzle.IA_ExitPuzzle"))
  (CallFunction|ReturntoCharacter))

(event Input|EnhancedActionEvents|EnhancedInputActionIA_NavigateRight
  (params (ActionValue :type Boolean) (ElapsedSeconds :type Float%20%28double-precision%29) (TriggeredSeconds :type Float%20%28double-precision%29) (InputAction :type Input%20Action%20Object%20Reference :default "/Game/Input/InputActions/IA_NavigateRight.IA_NavigateRight"))
  (CallFunction|ChangeSelectedDisc true))

(event Input|EnhancedActionEvents|EnhancedInputActionIA_NavigateLeft
  (params (ActionValue :type Boolean) (ElapsedSeconds :type Float%20%28double-precision%29) (TriggeredSeconds :type Float%20%28double-precision%29) (InputAction :type Input%20Action%20Object%20Reference :default "/Game/Input/InputActions/IA_NavigateLeft.IA_NavigateLeft"))
  (CallFunction|ChangeSelectedDisc false))

(event Input|EnhancedActionEvents|EnhancedInputActionIA_NavigateUp
  (params (ActionValue :type Boolean) (ElapsedSeconds :type Float%20%28double-precision%29) (TriggeredSeconds :type Float%20%28double-precision%29) (InputAction :type Input%20Action%20Object%20Reference :default "/Game/Input/InputActions/IA_NavigateUp.IA_NavigateUp"))
  (Default|Rotate (CallFunction|GetSelectedDisc) false))

(event Input|EnhancedActionEvents|EnhancedInputActionIA_NavigateDown
  (params (ActionValue :type Boolean) (ElapsedSeconds :type Float%20%28double-precision%29) (TriggeredSeconds :type Float%20%28double-precision%29) (InputAction :type Input%20Action%20Object%20Reference :default "/Game/Input/InputActions/IA_NavigateDown.IA_NavigateDown"))
  (Default|Rotate (CallFunction|GetSelectedDisc) true))

(event EventReturntoCharacter
  (|CallParentFunction)
  (CallFunction|SetSelectedDiscHighlight false))

(event EventBeginPlay
  (|CallParentFunction)
  (Variables|Default|SetDisc (Utilities|Array|MakeArray (Variables|Default|GetBP_Scheibe) (Variables|Default|GetBP_Scheibe1) (Variables|Default|GetBP_Scheibe2))))

(fn ConstructionScript)

(fn SetSelectedDiscHighlight
  (params (Enable :type Boolean))
  (CallFunction|SetHighlight Enable (CallFunction|GetSelectedDisc)))

(fn ChangeSelectedDisc
  (params (Right :type Boolean))
  (CallFunction|SetSelectedDiscHighlight false)
  (Variables|Default|SetSelectedDiscIndex (Math|Integer|Clamp(Integer) (+ (Variables|Default|GetSelectedDiscIndex) (Math|Integer|SelectInt 1 -1 Right)) 0 (Utilities|Array|LastIndex (Variables|Default|GetDisc))))
  (CallFunction|SetSelectedDiscHighlight true))

(fn GetSelectedDisc
  (return (Utilities|Array|Get(acopy) (Variables|Default|GetDisc) (Variables|Default|GetSelectedDiscIndex))))

(fn EvaluateCombination
  (for (_array_element _array_index) (Variables|Default|GetDisc)
    (if (Utilities|Enum|NotEqual(Enum) (Default|GetCurrentSymbol _array_element) (Utilities|Array|Get(acopy) (Variables|Default|GetCorrectCombination) _array_index))
      (return false)))
  (return true))

(fn Interact
  (params (PlayerCharacter :type BP%20First%20Person%20Character%20Object%20Reference) (Pickup :type BP%20Pickup%20Actor%20Object%20Reference))
  (|CallParentFunction PlayerCharacter Pickup)
  (CallFunction|SetSelectedDiscHighlight true)
  (return false))