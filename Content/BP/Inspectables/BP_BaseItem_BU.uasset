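; BP_BaseItem_BU is a base item Blueprint for inspectable props, configured through mesh, scale, name, description and inspection transform variables.
; The construction script applies the chosen mesh and world scale to its StaticMesh component.
; Interact is empty; the inspection logic is disconnected and never runs.
; That logic would spawn a BP_InspectItem far from the origin and pass it the mesh, text, rotation and scale.
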(event EventInteract
  (params (PlayerCharacter :type BP%20First%20Person%20Character%20Object%20Reference)))

(fn ConstructionScript
  (bind _static_mesh (Variables|Default|GetStatic%20Mesh))
  (Components|StaticMesh|SetStaticMesh (Variables|Default|GetStatic%20Mesh) (Variables|Default|GetItemMesh))
  (Transformation|SetWorldTransform (Variables|Default|GetStatic%20Mesh) (Math|Transform|MakeTransform (Transformation|GetWorldLocation _static_mesh) (Transformation|GetWorldRotation _static_mesh) (Variables|Default|GetItemScale)) false false))