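; Base Blueprint for inspectable items, which opens an inspection of the item when a player interacts with it.
; The construction script applies the configured mesh and world scale to its static mesh component.
; On Interact, if Inspected is true, it spawns a BP_InspectItem far outside the playable space.
; It passes that actor the inspection rotation and scale, the player character, mesh, name and description.
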(event EventInteract
  (params (PlayerCharacter :type BP%20First%20Person%20Character%20Object%20Reference))
  (if (Variables|Default|GetInspected)
    (bind _returnvalue (Game|SpawnActorfromClass "/Game/BP/Inspectables/BP_InspectItem.BP_InspectItem_C" (Math|Transform|MakeTransform "100000000.000000,0.000000,0.000000") "Undefined" "MultiplyWithRoot" 0 0))
    (Default|SetInspectRotation _returnvalue (Variables|Default|GetItemInspectionRotation))
    (Default|SetInspectScale _returnvalue (Variables|Default|GetItemInspectionScale))
    (Class|BPIInteractionInterface|Inspect(Message) _returnvalue PlayerCharacter (Variables|/Script/Engine.StaticMeshComponent|GetStaticMesh (Variables|Default|GetStatic%20Mesh)) (Variables|Default|GetItemName) (Variables|Default|GetItemDescription))))

(fn ConstructionScript
  (bind _static_mesh (Variables|Default|GetStatic%20Mesh))
  (Components|StaticMesh|SetStaticMesh (Variables|Default|GetStatic%20Mesh) (Variables|Default|GetItemMesh))
  (Transformation|SetWorldTransform (Variables|Default|GetStatic%20Mesh) (Math|Transform|MakeTransform (Transformation|GetWorldLocation _static_mesh) (Transformation|GetWorldRotation _static_mesh) (Variables|Default|GetItemScale)) false false))