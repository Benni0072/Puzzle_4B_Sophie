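; BP_Drawers is an interactable drawer that slides open and closed when Interact is triggered.
; Interact toggles the Open flag, and opening records the mesh's current relative location and sets an end point offset along local X.
; The OpenDrawer timeline lerps Cube012 between those points, playing from the start to open and reversing from the end to close.
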(event EventInteract
  (params (PlayerCharacter :type BP%20First%20Person%20Character%20Object%20Reference))
  (bind _cube_012 (Variables|Default|GetCube_012))
  (bind _relativelocation (Variables|/Script/Engine.SceneComponent|GetRelativeLocation _cube_012))
  (if (Variables|Default|GetOpen)
    (Variables|Default|SetOpen false)
    (Variables|Default|SetNewVar -3e+01)
    (bind _opendrawer (Timeline|Open%20Drawer ReverseFromEnd)
      (:Update
        (Transformation|SetRelativeLocation (Variables|Default|GetCube_012) (Math|Vector|Lerp(Vector) (Variables|Default|GetStartLocation) (Variables|Default|GetEndLocation) _opendrawer) false false)))
    (else
      (Variables|Default|SetOpen true)
      (Variables|Default|SetNewVar 3e+01)
      (Variables|Default|SetStartLocation (Math|Vector|MakeVector (.x _relativelocation) (.y _relativelocation) (.z _relativelocation)))
      (Variables|Default|SetEndLocation (Math|Vector|MakeVector (+ (.x _relativelocation) (Variables|Default|GetNewVar)) (.y _relativelocation) (.z _relativelocation)))
      (Timeline|Open%20Drawer PlayFromStart))))

(fn ConstructionScript)