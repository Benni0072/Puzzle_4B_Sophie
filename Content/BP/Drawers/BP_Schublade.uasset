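; Interactable drawer (Schublade) that slides a Cube component open and closed along the X axis.
; Interact toggles the Open state and calls MoveDrawer, which plays or reverses the OpenClose timeline to lerp the Cube's relative location.
; Endpoints derive from the Scene component's relative location on opening, and CanOpen acts as a busy lock until the timeline finishes.
; Interact flips Open even while that lock blocks movement.
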(event Custom|MoveDrawer
  (bind _scene (Variables|Default|GetScene))
  (bind _relativelocation (Variables|/Script/Engine.SceneComponent|GetRelativeLocation _scene))
  (if (not (Variables|Default|GetCanOpen?))
    (Variables|Default|SetCanOpen? true)
    (if (Variables|Default|GetOpen?)
      (Variables|Default|SetOpen? true)
      (Development|PrintString "Open")
      (Variables|Default|SetMoveDistance 3e+01)
      (Variables|Default|SetStartLocation (Math|Vector|MakeVector (.x _relativelocation) (.y _relativelocation) (.z _relativelocation)))
      (Variables|Default|SetEndLocation (Math|Vector|MakeVector (+ (.x _relativelocation) (Variables|Default|GetMoveDistance)) (.y _relativelocation) (.z _relativelocation)))
      (bind _newtrack_0 (Timeline|Open/Close Play)
        (:Update
          (Transformation|SetRelativeLocation (Variables|Default|GetCube) (Math|Vector|Lerp(Vector) (Variables|Default|GetStartLocation) (Variables|Default|GetEndLocation) _newtrack_0) false false))
        (:Finished
          (Variables|Default|SetCanOpen? false)))
      (else
        (Variables|Default|SetOpen? false)
        (Development|PrintString "Closed")
        (Variables|Default|SetMoveDistance -3e+01)
        (Timeline|Open/Close Reverse)))))

(fn ConstructionScript)

(fn Interact
  (params (PlayerCharacter :type BP%20First%20Person%20Character%20Object%20Reference) (Pickup :type BP%20Pickup%20Actor%20Object%20Reference))
  (Variables|Default|SetPlayer%20Character PlayerCharacter)
  (if (Variables|Default|GetOpen?)
    (Variables|Default|SetOpen? false)
    (else
      (Variables|Default|SetOpen? true)))
  (CallFunction|MoveDrawer)
  (return false))