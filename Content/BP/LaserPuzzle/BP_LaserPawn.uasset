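; BP_LaserPawn is a laser puzzle piece that emits a Niagara beam, starting lit if flagged as a laser source.
; While lit, it line-traces forward each tick and sets the beam length to the hit distance, or zero on a miss.
; A hit on another laser pawn's Box switches that pawn on, chaining beams.
; Nothing switches a lit pawn off after BeginPlay.
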(event Custom|GetHitByLasser
  (params (HitComponent :type Primitive%20Component%20Object%20Reference))
  ;[0.15 0.15 0.15 0.5] Recive Laser
  (if (== HitComponent (Variables|Default|GetBox))
    (CallFunction|SetLaserEnabled true)))

(event EventTick
  (params (DeltaSeconds :type Float%20%28single-precision%29))
  ;[0.15 0.15 0.15 0.5] EmitLaser
  (if (Variables|Default|GetLaser%20Is%20Enabled)
    (bind (_returnvalue _distancetohit _hitcomponent _hitlaserpossessable) (CallFunction|CheckforLaserHit))
    (if true
      (Niagara|SetNiagaraVariable(Float) (Variables|Default|GetNS_Laser) "LaserLength" _distancetohit)
      (Utilities|IsValid _hitlaserpossessable
        (:Is%20Valid
          (CallFunction|GetHitbyLasser _hitlaserpossessable _hitcomponent))))))

(event EventBeginPlay
  (CallFunction|SetLaserEnabled (Variables|Default|GetIsLaserSource)))

(fn ConstructionScript
  (|CallParentFunction))

(fn CheckforLaserHit
  (bind _ns_laser (Variables|Default|GetNS_Laser))
  (bind _returnvalue (Transformation|GetWorldLocation _ns_laser))
  (bind (_outhit _returnvalue_2) (Collision|LineTraceForObjects _returnvalue (+ _returnvalue (* (Math|Vector|GetForwardVector _ns_laser) (Variables|Default|GetMaxLaserRange))) (Utilities|Array|MakeArray "ObjectTypeQuery1" "ObjectTypeQuery2" "ObjectTypeQuery3" "ObjectTypeQuery4") false 0 "None"))
  (if _returnvalue_2
    (bind _asbp_laser_pawn (Utilities|Casting|CastToBP_LaserPawn (.HitActor (Collision|BreakHitResult _outhit)))
      (:then
        _)
      (:CastFailed
        _))
    (return true (Math|Vector|VectorLength (- (.ImpactPoint (Collision|BreakHitResult _outhit)) (Transformation|GetWorldLocation (Variables|Default|GetNS_Laser)))) (.HitComponent (Collision|BreakHitResult _outhit)) _asbp_laser_pawn)
    (else
      (return false 0.0 0 0))))

(fn SetLaserEnabled
  (params (IsEnabled :type Boolean))
  (bind _ns_laser (Variables|Default|GetNS_Laser))
  (bind _output_get (Variables|Default|SetLaser%20Is%20Enabled IsEnabled))
  (if _output_get
    (Components|Activation|Activate _ns_laser false)
    (else
      (Components|Activation|Deactivate _ns_laser))))