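; Interactable rotation puzzle Blueprint with three discs (Scheiben) that the player selects between after interacting, until exiting back to the character.
; Left and right inputs step the selected index with wrap-around over the disc array, moving a highlight overlay material to the current disc.
; Interact and return extend parent logic to toggle the highlight.
; Up and down inputs are empty, and the only rotation call is unconnected, so discs never rotate here.
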(event Input|EnhancedActionEvents|EnhancedInputActionIA_NavigateUp
  (params (ActionValue :type Boolean) (ElapsedSeconds :type Float%20%28double-precision%29) (TriggeredSeconds :type Float%20%28double-precision%29) (InputAction :type Input%20Action%20Object%20Reference :default "/Game/Input/InputActions/IA_NavigateUp.IA_NavigateUp")))

(event Input|EnhancedActionEvents|EnhancedInputActionIA_ExitPuzzle
  (params (ActionValue :type Boolean) (ElapsedSeconds :type Float%20%28double-precision%29) (TriggeredSeconds :type Float%20%28double-precision%29) (InputAction :type Input%20Action%20Object%20Reference :default "/Game/Input/InputActions/IA_ExitPuzzle.IA_ExitPuzzle"))
  (CallFunction|ReturntoCharacter))

(event Input|EnhancedActionEvents|EnhancedInputActionIA_NavigateRight
  (params (ActionValue :type Boolean) (ElapsedSeconds :type Float%20%28double-precision%29) (TriggeredSeconds :type Float%20%28double-precision%29) (InputAction :type Input%20Action%20Object%20Reference :default "/Game/Input/InputActions/IA_NavigateRight.IA_NavigateRight"))
  (CallFunction|NavigateButtons 1))

(event Input|EnhancedActionEvents|EnhancedInputActionIA_NavigateDown
  (params (ActionValue :type Boolean) (ElapsedSeconds :type Float%20%28double-precision%29) (TriggeredSeconds :type Float%20%28double-precision%29) (InputAction :type Input%20Action%20Object%20Reference :default "/Game/Input/InputActions/IA_NavigateDown.IA_NavigateDown")))

(event Input|EnhancedActionEvents|EnhancedInputActionIA_NavigateLeft
  (params (ActionValue :type Boolean) (ElapsedSeconds :type Float%20%28double-precision%29) (TriggeredSeconds :type Float%20%28double-precision%29) (InputAction :type Input%20Action%20Object%20Reference :default "/Game/Input/InputActions/IA_NavigateLeft.IA_NavigateLeft"))
  (CallFunction|NavigateButtons -1))

(event EventInteract
  (params (PlayerCharacter :type BP%20First%20Person%20Character%20Object%20Reference))
  (|CallParentFunction PlayerCharacter)
  (CallFunction|UpdateHighlightOfSelectedButton true))

(event EventReturntoCharacter
  (|CallParentFunction)
  (CallFunction|UpdateHighlightOfSelectedButton false))

(event EventBeginPlay
  (Variables|Default|SetRotScheibe (Utilities|Array|MakeArray (Variables|Default|GetBP_Scheibe) (Variables|Default|GetBP_Scheibe1) (Variables|Default|GetBP_Scheibe2))))

(fn ConstructionScript)

(fn UpdateHighlightOfSelectedButton
  (params (Enable :type Boolean))
  (Rendering|Material|SetOverlayMaterial (CallFunction|GetSelectedButton) (select Enable "/Game/Material/MM_Highlight_Inst.MM_Highlight_Inst" 0) :!class /Script/Engine.MeshComponent))

(fn NavigateButtons
  (params (Direction :type Integer))
  (CallFunction|UpdateHighlightOfSelectedButton false)
  (Variables|Default|SetCurrentScheibe (+ (Variables|Default|GetCurrentScheibe) Direction))
  (Utilities|FlowControl|Sequence
    (:then_0
      ;[1 1 1] Check if to high
      (if (> (Variables|Default|GetCurrentScheibe) (Utilities|Array|LastIndex (Variables|Default|GetRotScheibe)))
        (Variables|Default|SetCurrentScheibe (- (Variables|Default|GetCurrentScheibe) (Utilities|Array|Length (Variables|Default|GetRotScheibe))))))
    (:then_1
      ;[1 1 1] Check if to low
      (if (< (Variables|Default|GetCurrentScheibe) 0)
        (Variables|Default|SetCurrentScheibe (+ (Variables|Default|GetCurrentScheibe) (Utilities|Array|Length (Variables|Default|GetRotScheibe))))))
    (:then_2
      ;[1 1 1] Update Highlight
      (CallFunction|UpdateHighlightOfSelectedButton true))))

(fn GetSelectedButton
  (return (Utilities|Array|Get(acopy) (Variables|Default|GetRotScheibe) (Variables|Default|GetCurrentScheibe))))