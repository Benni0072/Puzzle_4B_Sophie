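; BP_HealthComponent is a health component that tracks damage and signals its owner's death.
; CurrentHealth starts at MaxHealt on BeginPlay, and TakeDamage subtracts the damage amount, then calls Die when IsHealthDepleted returns true, firing the OnDeath dispatcher.
; IsHealthDepleted tests CurrentHealth >= 0, so as written it reports depletion while health remains and not once it drops below zero.
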(event Custom|TakeDamage
  (params (DamageAmount :type Float%20%28double-precision%29))
  (Variables|Default|SetCurrentHealth (- (Variables|Default|GetCurrentHealth) DamageAmount))
  (if (CallFunction|IsHealthDepleted)
    (CallFunction|Die)))

(event Custom|Die
  (Default|CallOnDeath))

(event EventBeginPlay
  (Variables|Default|SetCurrentHealth (Variables|Default|GetMaxHealt)))

(fn IsHealthDepleted
  (return (>= (Variables|Default|GetCurrentHealth) 0.0)))